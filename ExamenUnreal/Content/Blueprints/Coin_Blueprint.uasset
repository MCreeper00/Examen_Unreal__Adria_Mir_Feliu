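; Coin pickup actor that adds one to the ThirdPersonCharacter's Coins count when that character overlaps it, then destroys itself.
; The SoundCoin boolean on the character flips on each pickup, alternating between the Coin and Coin2 sounds across coins.
; Both sounds play at a random pitch, but only Coin2 is given the Sphere's world location.
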(event `self.ReceiveActorBeginOverlap`
  (params (OtherActor :type "Actor Object Reference"))
  (bind _returnvalue (`KismetMathLibrary.RandomFloat`))
  (bind _asthird_person_character (cast `/Game/ThirdPersonBP/Blueprints/ThirdPersonCharacter` OtherActor))
  (bind _result (`/Engine/EditorBlueprintResources/StandardMacros.IncrementInt` (`/Game/ThirdPersonBP/Blueprints/ThirdPersonCharacter.Coins` _asthird_person_character))
    (:`  `
      (set `/Game/ThirdPersonBP/Blueprints/ThirdPersonCharacter.Coins` _result _asthird_person_character)
      (if (`/Game/ThirdPersonBP/Blueprints/ThirdPersonCharacter.SoundCoin` _asthird_person_character)
        (`GameplayStatics.PlaySoundAtLocation` "/Game/Sound/coin.coin" (0.0 0.0 0.0) (struct) 1.0 _returnvalue 0.0 null null null)
        (else
          (`GameplayStatics.PlaySoundAtLocation` "/Game/Sound/coin2.coin2" (`SceneComponent.K2_GetComponentLocation` (`self.Sphere`)) (struct) 1.0 _returnvalue 0.0 null null null)))
      (bind _output_get (set `/Game/ThirdPersonBP/Blueprints/ThirdPersonCharacter.SoundCoin` (not (stale _output_get)) _asthird_person_character))
      (`self.K2_DestroyActor`))))

(fn `UserConstructionScript`)